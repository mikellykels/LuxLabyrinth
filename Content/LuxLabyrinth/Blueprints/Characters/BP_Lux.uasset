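; BP_Lux is the Lux Labyrinth character Blueprint that sets up the player's HUD and hands off from tutorial instructions to the main quest.
; On BeginPlay it creates health bar and instructions widgets, then binds to the instructions' completion event.
; When instructions complete, it waits briefly, removes them, gets the hoop count HUD from the game mode, sets the hoop-lighting quest text and shows it.
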(event Custom|HandleInstructionsCompleted
  (Utilities|FlowControl|Delay 1.0)
  (Widget|RemovefromParent (Variables|Default|GetInstructionsHUD))
  (bind _asbp_lux_labyrinth_game_mode (Utilities|Casting|CastToBP_LuxLabyrinthGameMode (Game|GetGameMode)))
  (bind _output_get (Variables|Default|SetGameMode _asbp_lux_labyrinth_game_mode))
  (bind _aswbp_lux_labyrinth_hoop_count_hud (Utilities|Casting|CastToWBP_LuxLabyrinthHoopCountHUD (Class|LuxLabyrinthGameMode|GetHoopHud _output_get)))
  (bind _output_get_2 (Variables|Default|SetHoopHUD _aswbp_lux_labyrinth_hoop_count_hud))
  (Class|LuxLabyrinthHoopCountHUD|UpdateMainQuestText _output_get_2 "Pass through hoops to light up a section")
  (Widget|SetVisibility (Class|LuxLabyrinthGameMode|GetHoopHud _output_get) "Visible"))

(event EventBeginPlay
  (Utilities|FlowControl|Sequence
    (:then_0
      (bind _returnvalue (UserInterface|CreateWidget "/Game/LuxLabyrinth/Blueprints/UI/WBP_LuxLabyrinthHealthBarHUD.WBP_LuxLabyrinthHealthBarHUD_C"))
      (bind _output_get (Variables|Default|SetHealthBarHUD _returnvalue))
      (UserInterface|Viewport|AddtoViewport _output_get 0))
    (:then_1
      (bind _returnvalue_2 (UserInterface|CreateWidget "/Game/LuxLabyrinth/Blueprints/UI/WBP_LuxLabyrinthInstructionsHUD.WBP_LuxLabyrinthInstructionsHUD_C"))
      (bind _output_get_2 (Variables|Default|SetInstructionsHUD _returnvalue_2))
      (UserInterface|Viewport|AddtoViewport _output_get_2 0))
    (:then_2
      (EventDispatchers|BindEventtoOnAllInstructionsCompleted (Variables|Default|GetInstructionsHUD) (delegate Custom|HandleInstructionsCompleted)))))

(fn ConstructionScript)